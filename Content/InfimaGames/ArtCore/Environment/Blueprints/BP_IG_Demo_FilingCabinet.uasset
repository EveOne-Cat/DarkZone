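; Filing cabinet demo environment prop that randomizes the look of its four drawers.
; The construction script runs UpdateDrawer on each drawer component, giving it a one-in-three chance to be hidden and sliding it out along local Y by a random amount.
; It uses unseeded randomness, so drawers re-roll whenever construction reruns, and it has no runtime logic.
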(event EventBeginPlay)

(event Collision|EventActorBeginOverlap
  (params (OtherActor :type Actor%20Object%20Reference)))

(event EventTick
  (params (DeltaSeconds :type Float%20%28single-precision%29)))

(fn ConstructionScript
  (CallFunction|UpdateDrawer (Variables|Default|GetDrawer_01))
  (CallFunction|UpdateDrawer (Variables|Default|GetDrawer_02))
  (CallFunction|UpdateDrawer (Variables|Default|GetDrawer_03))
  (CallFunction|UpdateDrawer (Variables|Default|GetDrawer_04)))

(fn UpdateDrawer
  (params (Target :type Scene%20Component%20Object%20Reference))
  (Utilities|FlowControl|Sequence
    (:then_0
      (if (== (Math|Random|RandomIntegerinRange 1 3) 1)
        (Rendering|SetVisibility Target false false) ; Hide
        (else
          (Rendering|SetVisibility Target true false) ; Show
        ))
      (Transformation|AddLocalOffset Target (Math|Vector|MakeVector 0.0 (Math|Random|RandomFloatinRange 0.0 2e+01) 0.0) false false) ; Drawer out
    )
    (:then_1
      (return))))