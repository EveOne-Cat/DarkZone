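; Animation notify that updates the gameplay ability tags on the mesh's owning actor when an animation reaches it.
; It reads the owner's tags through interface messages, adds TagsAdded uniquely, removes TagsRemoved, then writes the result back.
; ForceSetAll swaps the added list for a hardcoded set of tags and renames the notify "Fill Tags".
; RunForAI limits the update to owners that report as AI.
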(fn ReceivedNotify
  (params (MeshComp :type Skeletal%20Mesh%20Component%20Object%20Reference) (Animation :type Anim%20Sequence%20Base%20Object%20Reference) (EventReference :type Anim%20Notify%20Event%20Reference%20Structure%20%28by%20ref%29))
  (bind _returnvalue (Components|GetOwner MeshComp))
  (Utilities|FlowControl|Sequence
    (:then_0
      (Utilities|IsValid MeshComp
        (:Is%20Valid
          (if (Variables|Default|GetRun%20For%20AI)
            (bind _returnvalue_2 (Class|BPIIGCharacter|IsAI(Message) _returnvalue))
            (if _returnvalue_2
              (bind _tags (Class|BPIIGCharacter|GetGameAbilityTags(Message) _returnvalue :!label _label))
              (LocalVariables|SetTags _tags)
              (for _array_element (select (Variables|Default|GetForce%20Set%20All) (Utilities|Array|MakeArray "NewEnumerator0" "NewEnumerator1" "NewEnumerator2" "NewEnumerator3" "NewEnumerator4" "NewEnumerator5" "NewEnumerator6" "NewEnumerator7" "NewEnumerator8" "NewEnumerator9" "NewEnumerator10" "NewEnumerator11" "NewEnumerator12" "NewEnumerator13" "NewEnumerator14" "NewEnumerator15" "NewEnumerator16" "NewEnumerator18" "NewEnumerator35" "NewEnumerator37" "NewEnumerator41") (Variables|Default|GetTags%20Added))
                (Utilities|Array|AddUnique (LocalVariables|GetTags) _array_element))
              (for _array_element_2 (Variables|Default|GetTags%20Removed)
                (Utilities|Array|RemoveItem (LocalVariables|GetTags) _array_element_2))
              (Class|BPIIGCharacter|SetGameAbilityTags(Message) (Components|GetOwner MeshComp) (LocalVariables|GetTags)))
            (else
              (goto _label))))))
    (:then_1
      (return true))))

(fn GetNotifyName
  (return (select (Variables|Default|GetForce%20Set%20All) "Fill Tags" "Update Tags")))