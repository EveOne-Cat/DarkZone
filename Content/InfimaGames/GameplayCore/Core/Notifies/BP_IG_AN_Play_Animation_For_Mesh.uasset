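; Anim notify that plays a montage on another skeletal mesh of the owning actor, picked by component tag.
; It takes the first component matching MeshTag and, if its anim instance is valid, plays the montage, optionally stopping others.
; When RunForAI is set, an interface check skips AI owners; otherwise it plays for any owner.
; The notify's display name includes the target tag.
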(fn ReceivedNotify
  (params (MeshComp :type Skeletal%20Mesh%20Component%20Object%20Reference) (Animation :type Anim%20Sequence%20Base%20Object%20Reference) (EventReference :type Anim%20Notify%20Event%20Reference%20Structure%20%28by%20ref%29))
  (bind _mesh_tag (Variables|Default|GetMesh%20Tag))
  (bind _returnvalue (Components|GetOwner MeshComp))
  (bind _returnvalue_2 (Actor|GetComponentsbyTag _returnvalue "/Script/Engine.SkeletalMeshComponent" _mesh_tag))
  (bind _output (Utilities|Array|Get(acopy) _returnvalue_2))
  (bind _returnvalue_3 (Components|SkeletalMesh|GetAnimInstance _output))
  (Utilities|FlowControl|Sequence
    (:then_0
      (if (Variables|Default|GetRun%20For%20AI)
        (bind _returnvalue_4 (Class|BPIIGCharacter|IsAI(Message) (Components|GetOwner MeshComp)))
        (if (not _returnvalue_4)
          (Utilities|IsValid _output :!label _label
            (:Is%20Valid
              (Utilities|IsValid _returnvalue_3
                (:Is%20Valid
                  (Animation|Montage|MontagePlay _returnvalue_3 (Variables|Default|GetAnimation) 1.0 "MontageLength" 0.0 (Variables|Default|GetStop%20All%20Montages)))))))
        (else
          (goto _label))))
    (:then_1
      (return true))))

(fn GetNotifyName
  (return (Utilities|String|Append "Play Animation for Mesh: " (Utilities|String|ToString(Name) (Variables|Default|GetMesh%20Tag)))))