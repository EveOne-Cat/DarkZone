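; Animation notify that sets the visibility of the magazine on a character's equipped item during an animation.
; When fired, it gets the equipped item from the mesh's owner through a message call.
; If that item is valid, it sends a set-hidden-magazine message carrying the notify's Hidden value.
; It displays in the animation timeline as "Set Character Equipped Magazine Hidden".
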(fn ReceivedNotify
  (params (MeshComp :type Skeletal%20Mesh%20Component%20Object%20Reference) (Animation :type Anim%20Sequence%20Base%20Object%20Reference) (EventReference :type Anim%20Notify%20Event%20Reference%20Structure%20%28by%20ref%29))
  (Utilities|FlowControl|Sequence
    (:then_0
      (Utilities|IsValid (Components|GetOwner MeshComp)
        (:Is%20Valid
          (bind _equipped_item (Class|BPIIGCharacter|GetEquippedItem(Message) (Components|GetOwner MeshComp)))
          (Utilities|IsValid _equipped_item
            (:Is%20Valid
              (Class|BPIIGWeapon|OnSetHiddenMagazine(Message) _equipped_item (Variables|Default|GetHidden)))))))
    (:then_1
      (return true))))

(fn GetNotifyName
  (return "Set Character Equipped Magazine Hidden"))