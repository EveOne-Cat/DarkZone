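; Animation notify that shows or hides a tagged scene component on the animated mesh's owner.
; It takes the first component matching MeshTag and, if valid, applies the Show flag as visibility, propagating to children.
; When RunForAI is set, it queries the owner through IsAIMessage and skips owners reporting as AI; otherwise it always runs.
; The notify's display name includes the tag.
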(fn ReceivedNotify
  (params (MeshComp :type Skeletal%20Mesh%20Component%20Object%20Reference) (Animation :type Anim%20Sequence%20Base%20Object%20Reference) (EventReference :type Anim%20Notify%20Event%20Reference%20Structure%20%28by%20ref%29))
  (bind _mesh_tag (Variables|Default|GetMesh%20Tag))
  (bind _returnvalue (Components|GetOwner MeshComp))
  (bind _returnvalue_2 (Actor|GetComponentsbyTag _returnvalue "/Script/Engine.SceneComponent" _mesh_tag))
  (bind _output (Utilities|Array|Get(acopy) _returnvalue_2))
  (Utilities|FlowControl|Sequence
    (:then_0
      (if (Variables|Default|GetRun%20For%20AI)
        (bind _returnvalue_3 (Class|BPIIGCharacter|IsAI(Message) (Components|GetOwner MeshComp)))
        (if (not _returnvalue_3)
          (Utilities|IsValid _output :!label _label
            (:Is%20Valid
              (Rendering|SetVisibility _output (Variables|Default|GetShow) true))))
        (else
          (goto _label))))
    (:then_1
      (return true))))

(fn GetNotifyName
  (return (Utilities|String|Append "Set Visibility for Mesh: " (Utilities|String|ToString(Name) (Variables|Default|GetMesh%20Tag)))))