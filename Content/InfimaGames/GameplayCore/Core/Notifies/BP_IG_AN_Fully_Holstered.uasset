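; Animation notify, shown as "Fully Holstered", that tells the mesh owner's inventory component that it is fully holstered.
; On firing, it finds BPSC_IG_Inventory on the owning actor and sets the fully holstered state to true.
; When RunForAI is enabled, it does so only if the owner reports itself as AI through IsAIMessage.
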(fn ReceivedNotify
  (params (MeshComp :type Skeletal%20Mesh%20Component%20Object%20Reference) (Animation :type Anim%20Sequence%20Base%20Object%20Reference) (EventReference :type Anim%20Notify%20Event%20Reference%20Structure%20%28by%20ref%29))
  (bind _returnvalue (Components|GetOwner MeshComp))
  (bind _returnvalue_2 (Actor|GetComponentbyClass _returnvalue "/Game/InfimaGames/GameplayCore/Core/Inventory/BPSC_IG_Inventory.BPSC_IG_Inventory_C"))
  (Utilities|FlowControl|Sequence
    (:then_0
      (Utilities|IsValid MeshComp
        (:Is%20Valid
          (if (Variables|Default|GetRun%20For%20AI)
            (bind _returnvalue_3 (Class|BPIIGCharacter|IsAI(Message) (Components|GetOwner MeshComp)))
            (if _returnvalue_3
              (Utilities|IsValid _returnvalue_2 :!label _label
                (:Is%20Valid
                  (Default|EventSetFullyHolstered _returnvalue_2 true))))
            (else
              (goto _label))))))
    (:then_1
      (return true))))

(fn GetNotifyName
  (return "Fully Holstered"))