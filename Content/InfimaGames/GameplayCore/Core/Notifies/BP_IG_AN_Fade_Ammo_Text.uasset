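; Animation notify that fades a weapon's floating ammunition text in or out during an animation.
; On trigger, it takes the mesh's owner as the weapon, gets its ammo text message and casts it to the floating ammunition text widget.
; Its Fade flag picks the widget's fade-in or fade-out event, and it displays as "Fade Ammo Text".
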(fn ReceivedNotify
  (params (MeshComp :type Skeletal%20Mesh%20Component%20Object%20Reference) (Animation :type Anim%20Sequence%20Base%20Object%20Reference) (EventReference :type Anim%20Notify%20Event%20Reference%20Structure%20%28by%20ref%29))
  (Utilities|FlowControl|Sequence
    (:then_0
      (LocalVariables|SetWeapon (Components|GetOwner MeshComp))
      (bind _returnvalue (Class|BPIIGWeapon|GetAmmoText(Message) (LocalVariables|GetWeapon)))
      (bind _aswbp_ig_ammunition_text_floating (Utilities|Casting|CastToWBP_IG_Ammunition_Text_Floating _returnvalue))
      (if (Variables|Default|GetFade)
        (Default|EventFadein _aswbp_ig_ammunition_text_floating)
        (else
          (Default|EventFadeOut _aswbp_ig_ammunition_text_floating))))
    (:then_1
      (return true))))

(fn GetNotifyName
  (return "Fade Ammo Text"))