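; Animation notify that drops a physics magazine from a weapon, shown in the editor as "Drop Physics Magazine".
; It gets the magazine static mesh component from the animated mesh's owning weapon through a message call.
; If valid, it spawns a BP_IG_Mag_Drop actor at that component's transform, shifted by a location offset, and copies the static mesh so the dropped magazine matches the visual one.
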(fn ReceivedNotify
  (params (MeshComp :type Skeletal%20Mesh%20Component%20Object%20Reference) (Animation :type Anim%20Sequence%20Base%20Object%20Reference) (EventReference :type Anim%20Notify%20Event%20Reference%20Structure%20%28by%20ref%29))
  (Utilities|FlowControl|Sequence
    (:then_0
      (bind _output_get (LocalVariables|SetWeapon (Components|GetOwner MeshComp)))
      (bind _returnvalue (Class|BPIIGWeapon|GetStaticMeshMagazine(Message) _output_get))
      (bind _output_get_2 (LocalVariables|SetMag_Mesh _returnvalue))
      (Utilities|IsValid _output_get_2
        (:Is%20Valid
          (bind _returnvalue_2 (Game|SpawnActorfromClass "/Game/InfimaGames/GameplayCore/Core/Weapons/BP_IG_Mag_Drop.BP_IG_Mag_Drop_C" (Math|Transform|MakeTransform (Math|Transform|TransformLocation (Transformation|GetWorldTransform (LocalVariables|GetMag_Mesh)) (Variables|Default|GetLocation%20Offset)) (.Rotation (Math|Transform|BreakTransform (Transformation|GetWorldTransform (LocalVariables|GetMag_Mesh)))) (.Scale (Math|Transform|BreakTransform (Transformation|GetWorldTransform (LocalVariables|GetMag_Mesh))))) "AlwaysSpawn" 0 0 :!pinned true)) ; Spawn New Magazine. This drops the magazine, basically.
          (LocalVariables|SetDropped _returnvalue_2)
          (Components|StaticMesh|SetStaticMesh (Variables|/Game/InfimaGames/GameplayCore/Core/Weapons/BP_IG_Mag_Drop.BP_IG_Mag_Drop_C|GetMagazine (LocalVariables|GetDropped)) (Variables|/Script/Engine.StaticMeshComponent|GetStaticMesh (LocalVariables|GetMag_Mesh)) :!pinned true) ; Copy Static Mesh. Matches the visual magazine.
        )))
    (:then_1
      (return true))))

(fn GetNotifyName
  (return "Drop Physics Magazine"))