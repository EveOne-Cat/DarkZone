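; Anim notify, shown as "Completed Bolt Action", that updates the bolt state of the owning character's equipped item.
; It gets the equipped item from the mesh owner through message calls and, if valid, sends it a fixed bolt-state value.
; When RunForAI is set, the update only happens if the owner reports itself as AI; otherwise it runs for any owner.
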(fn ReceivedNotify
  (params (MeshComp :type Skeletal%20Mesh%20Component%20Object%20Reference) (Animation :type Anim%20Sequence%20Base%20Object%20Reference) (EventReference :type Anim%20Notify%20Event%20Reference%20Structure%20%28by%20ref%29))
  (Utilities|FlowControl|Sequence
    (:then_0
      (if (Variables|Default|GetRun%20For%20AI)
        (bind _returnvalue (Class|BPIIGCharacter|IsAI(Message) (Components|GetOwner MeshComp)))
        (if _returnvalue
          (bind _equipped_item (Class|BPIIGCharacter|GetEquippedItem(Message) (Components|GetOwner MeshComp) :!label _label))
          (Utilities|IsValid _equipped_item
            (:Is%20Valid
              (Class|BPIIGWeapon|OnSetBoltState(Message) _equipped_item "NewEnumerator0"))))
        (else
          (goto _label))))
    (:then_1
      (return true))))

(fn GetNotifyName
  (return "Completed Bolt Action"))