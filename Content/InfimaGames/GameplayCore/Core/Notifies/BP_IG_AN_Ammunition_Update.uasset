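; Animation notify that updates ammunition at a chosen point in an animation, shown in the editor as "Update Ammunition".
; It sends an OnAmmunitionSet message carrying its Fill and Amount properties to the mesh owner's attach parent actor, or to the owner itself when no valid parent exists.
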(fn ReceivedNotify
  (params (MeshComp :type Skeletal%20Mesh%20Component%20Object%20Reference) (Animation :type Anim%20Sequence%20Base%20Object%20Reference) (EventReference :type Anim%20Notify%20Event%20Reference%20Structure%20%28by%20ref%29))
  (Utilities|FlowControl|Sequence
    (:then_0
      (Utilities|IsValid (Actor|GetAttachParentActor (Components|GetOwner MeshComp))
        (:Is%20Valid
          (Class|BPIIGCharacter|OnAmmunitionSet(Message) (Actor|GetAttachParentActor (Components|GetOwner MeshComp)) (Variables|Default|GetFill) (Variables|Default|GetAmount)))
        (:Is%20Not%20Valid
          (Class|BPIIGCharacter|OnAmmunitionSet(Message) (Components|GetOwner MeshComp) (Variables|Default|GetFill) (Variables|Default|GetAmount)))))
    (:then_1
      (return true))))

(fn GetNotifyName
  (return "Update Ammunition"))