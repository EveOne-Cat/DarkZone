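; Anim notify, displayed as "Melee", that triggers a melee act on the animated mesh's owner.
; It finds the owner's BPAC_IG_PCH_Melee component and calls EventAct when that component is valid.
; When RunForAI is set, it first queries the owner through IsAIMessage and only acts for AI; otherwise it acts for any owner.
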(fn ReceivedNotify
  (params (MeshComp :type Skeletal%20Mesh%20Component%20Object%20Reference) (Animation :type Anim%20Sequence%20Base%20Object%20Reference) (EventReference :type Anim%20Notify%20Event%20Reference%20Structure%20%28by%20ref%29))
  (Utilities|FlowControl|Sequence
    (:then_0
      (if (Variables|Default|GetRun%20For%20AI)
        (bind _returnvalue (Class|BPIIGCharacter|IsAI(Message) (Components|GetOwner MeshComp)))
        (if _returnvalue
          (bind _output_get (LocalVariables|SetMelee%20Component (Actor|GetComponentbyClass (Components|GetOwner MeshComp) "/Game/InfimaGames/GameplayCore/Core/Characters/BPAC_IG_PCH_Melee.BPAC_IG_PCH_Melee_C") :!label _label))
          (Utilities|IsValid _output_get
            (:Is%20Valid
              (Default|EventAct (LocalVariables|GetMelee%20Component)))))
        (else
          (goto _label))))
    (:then_1
      (return true))))

(fn GetNotifyName
  (return "Melee"))