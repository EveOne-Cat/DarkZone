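; Tutorial trigger actor that shows a tutorial widget while a Character is inside its Shape and fades it out once none remain.
; Tick polls the Shape for overlapping Characters rather than using overlap events.
; Two cross-reset DoOnce gates turn the poll into enter and exit edges: entry creates the configured Widget class for player 0, and exit calls EventFadeOut on that instance.
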(event EventTick
  (params (DeltaSeconds :type Float%20%28single-precision%29))
  (|CallParentFunction DeltaSeconds)
  (if (> (Utilities|Array|Length (Collision|GetOverlappingActors (Variables|Default|GetShape) "/Script/Engine.Character" :!class /Script/Engine.PrimitiveComponent)) 0)
    (Utilities|FlowControl|Sequence
      (:then_0
        (Utilities|FlowControl|DoOnce false :!label _label
          (:Completed
            (if (Utilities|IsValidClass (Variables|Config|GetWidget))
              (bind _returnvalue (UserInterface|CreateWidget (Variables|Config|GetWidget) (Game|GetPlayerController 0)))
              (Variables|Data|SetWidget%20Reference _returnvalue)
              (UserInterface|Viewport|AddtoViewport _returnvalue 0)))))
      (:then_1
        (goto _label_2 Reset)))
    (else
      (Utilities|FlowControl|Sequence
        (:then_0
          (Utilities|FlowControl|DoOnce false :!label _label_2
            (:Completed
              (Utilities|IsValid (Variables|Data|GetWidget%20Reference)
                (:Is%20Valid
                  (Default|EventFadeOut (Variables|Data|GetWidget%20Reference)))))))
        (:then_1
          (goto _label Reset))))))

(fn ConstructionScript)