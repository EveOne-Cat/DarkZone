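; Tutorial manager that gates a course with start, end and reset triggers, responding only to the assault rifle player.
; The start trigger turns both lights red, shows the start door and hides the end door, while the end trigger turns its light green and shows the end door.
; Reset, by trigger or event, re-arms the start, turns its light green and hides both start doors.
; Doors toggle through visibility and collision, with flags preventing repeat triggers.
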(event OnActorBeginOverlap(TriggerStart)
  (params (OverlappedActor :type Actor%20Object%20Reference) (OtherActor :type Actor%20Object%20Reference))
  (bind _door_end (Variables|Default|GetDoor%20End))
  (bind _staticmeshcomponent (Variables|/Script/Engine.StaticMeshActor|GetStaticMeshComponent _door_end))
  (Utilities|Casting|CastToBP_RAR_AssaultRifle_Player OtherActor)
  (if (not (Variables|Default|GetTriggeredStart))
    (Rendering|Components|Light|SetLightColor (Variables|/Script/Engine.Light|GetLightComponent (Variables|Default|GetLight%20Start)) "(R=1.000000,G=0.004391,B=0.000000,A=1.000000)" true)
    (Variables|Default|SetTriggeredStart true)
    (Rendering|SetVisibility (Variables|/Script/Engine.StaticMeshActor|GetStaticMeshComponent (Variables|Default|GetDoor%20Start)) true false)
    (Collision|SetCollisionEnabled (Variables|/Script/Engine.StaticMeshActor|GetStaticMeshComponent (Variables|Default|GetDoor%20Start)) "QueryOnly")
    (Audio|PlaySoundatLocation "/Game/InfimaGames/ArtCore/Audio/_Common/SC_IG_Demo_LightSwitch.SC_IG_Demo_LightSwitch" (Transformation|GetWorldLocation (Variables|/Script/Engine.Light|GetLightComponent (Variables|Default|GetLight%20Start))) "0, 0, 0" 1.0 1.0 0.0 0 0 0 0)
    (Rendering|SetVisibility _staticmeshcomponent false false)
    (Collision|SetCollisionEnabled _staticmeshcomponent "NoCollision")
    (Variables|Default|SetTriggeredEnd false)
    (Rendering|Components|Light|SetLightColor (Variables|/Script/Engine.Light|GetLightComponent (Variables|Default|GetLight%20End)) "(R=1.000000,G=0.004391,B=0.000000,A=1.000000)" true)))

(event OnActorBeginOverlap(TriggerReset)
  (params (OverlappedActor :type Actor%20Object%20Reference) (OtherActor :type Actor%20Object%20Reference))
  (Utilities|Casting|CastToBP_RAR_AssaultRifle_Player OtherActor)
  (Variables|Default|SetTriggeredStart false)
  (Rendering|Components|Light|SetLightColor (Variables|/Script/Engine.Light|GetLightComponent (Variables|Default|GetLight%20Start)) "(R=0.057805,G=1.000000,B=0.000000,A=1.000000)" true)
  (Rendering|SetVisibility (Variables|/Script/Engine.StaticMeshActor|GetStaticMeshComponent (Variables|Default|GetDoor%20Start)) false false)
  (Collision|SetCollisionEnabled (Variables|/Script/Engine.StaticMeshActor|GetStaticMeshComponent (Variables|Default|GetDoor%20Start%20Closed)) "NoCollision"))

(event OnActorBeginOverlap(TriggerEnd)
  (params (OverlappedActor :type Actor%20Object%20Reference) (OtherActor :type Actor%20Object%20Reference))
  (bind _light_end (Variables|Default|GetLight%20End))
  (bind _door_end (Variables|Default|GetDoor%20End))
  (bind _staticmeshcomponent (Variables|/Script/Engine.StaticMeshActor|GetStaticMeshComponent _door_end))
  (Utilities|Casting|CastToBP_RAR_AssaultRifle_Player OtherActor)
  (if (not (Variables|Default|GetTriggeredEnd))
    (Rendering|Components|Light|SetLightColor (Variables|/Script/Engine.Light|GetLightComponent _light_end) "(R=0.057805,G=1.000000,B=0.000000,A=1.000000)" true)
    (Variables|Default|SetTriggeredEnd true)
    (Rendering|SetVisibility _staticmeshcomponent true false)
    (Collision|SetCollisionEnabled _staticmeshcomponent "QueryOnly")
    (Audio|PlaySoundatLocation "/Game/InfimaGames/ArtCore/Audio/_Common/SC_IG_Demo_LightSwitch.SC_IG_Demo_LightSwitch" (Transformation|GetWorldLocation (Variables|/Script/Engine.Light|GetLightComponent _light_end)) "0, 0, 0" 1.0 1.0 0.0 0 0 0 0)))

(event Custom|Event%20Reset
  (Variables|Default|SetTriggeredStart false)
  (Rendering|Components|Light|SetLightColor (Variables|/Script/Engine.Light|GetLightComponent (Variables|Default|GetLight%20Start)) "(R=0.057805,G=1.000000,B=0.000000,A=1.000000)" true)
  (Rendering|SetVisibility (Variables|/Script/Engine.StaticMeshActor|GetStaticMeshComponent (Variables|Default|GetDoor%20Start)) false false)
  (Collision|SetCollisionEnabled (Variables|/Script/Engine.StaticMeshActor|GetStaticMeshComponent (Variables|Default|GetDoor%20Start%20Closed)) "NoCollision"))

(event EventBeginPlay
  ;[0.7044 1 0 1 12] Begin Play
  (Rendering|SetVisibility (Variables|/Script/Engine.StaticMeshActor|GetStaticMeshComponent (Variables|Default|GetDoor%20Start)) false false)
  (Collision|SetCollisionEnabled (Variables|/Script/Engine.StaticMeshActor|GetStaticMeshComponent (Variables|Default|GetDoor%20Start)) "NoCollision"))

(fn ConstructionScript)