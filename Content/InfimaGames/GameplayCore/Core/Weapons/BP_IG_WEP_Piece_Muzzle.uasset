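; Muzzle weapon piece Blueprint that provides a brief muzzle flash light.
; When its FlashLight event runs and flashes are enabled, it randomizes the Flash light's intensity and attenuation radius from configured ranges.
; It shows the light, then hides it after a short retriggerable delay, so repeated triggers extend the visible flash rather than stacking.
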(event Custom|Event%20Flash%20Light
  (if (Variables|Config|GetUses%20Flash)
    (Rendering|Components|Light|SetIntensity (Variables|Default|GetFlash) (CallFunction|RandomFloatinVectorRange (Variables|Config|GetIntensity%20Range)))
    (Rendering|Lighting|SetAttenuationRadius (Variables|Default|GetFlash) (CallFunction|RandomFloatinVectorRange (Variables|Config|GetRadius%20Range)))
    (Rendering|SetVisibility (Variables|Default|GetFlash) true false)
    (Utilities|FlowControl|RetriggerableDelay 0.05)
    (Rendering|SetVisibility (Variables|Default|GetFlash) false false)))

(fn ConstructionScript
  (|CallParentFunction))