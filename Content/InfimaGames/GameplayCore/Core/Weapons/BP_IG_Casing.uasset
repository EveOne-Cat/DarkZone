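; BP_IG_Casing is a weapon shell casing actor that flies out, spins, and destroys itself after a random delay.
; ApplyImpulse launches it through ProjectileMovement, adding the owner's velocity to the impulse, and a first hard bounce plays a sound once.
; Tick handles spin and lifetime, while mesh hits stop the spin.
; BeginPlay and hits set the material "Field Of View Alpha" parameter for first-person FOV rendering.
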(event OnComponentHit(Mesh)
  (params (HitComponent :type Primitive%20Component%20Object%20Reference) (OtherActor :type Actor%20Object%20Reference) (OtherComp :type Primitive%20Component%20Object%20Reference) (NormalImpulse :type Vector :default "0, 0, 0") (Hit :type Hit%20Result%20Structure%20%28by%20ref%29))
  (Rendering|Material|SetScalarParameterValueonMaterials (Variables|Default|GetMesh) "Field Of View Alpha" 0.0)
  (Variables|InfimaGames|Casing|SetRotate false))

(event OnProjectileBounce(ProjectileMovement)
  (params (ImpactResult :type Hit%20Result%20Structure%20%28by%20ref%29) (ImpactVelocity :type Vector%20%28by%20ref%29 :default "0, 0, 0"))
  (if (> (Math|Vector|VectorLength ImpactVelocity) 3e+02)
    (Utilities|FlowControl|DoOnce false
      (:Completed
        (Audio|PlaySoundatLocation (Variables|InfimaGames|Casing|GetSound) (Transformation|GetActorLocation) "0, 0, 0" 1.0 1.0 0.0 0 0 0 0)))))

(event Custom|Event%20Apply%20Impulse
  (params (Direction :type Vector) (Strength :type Vector))
  (Variables|/Script/Engine.MovementComponent|SetVelocity (Variables|Default|GetProjectile%20Movement) (+ (Transformation|GetVelocity (Components|GetOwner)) (* Direction Strength))))

(event EventBeginPlay
  (|CallParentFunction)
  (Variables|InfimaGames|Data|SetDestroy%20Delay (CallFunction|RandomFloatinVectorRange (Variables|InfimaGames|Casing|GetDestroy%20Delay%20Range)))
  (Rendering|Material|SetScalarParameterValueonMaterials (Variables|Default|GetMesh) "Field Of View Alpha" 0.0) ; This node makes sure that the casing actually uses a separate \nfirst-person field of view, just like the weapon and character do.\n\nNot having this here will make the spawned casings look like they're behind the\ncharacter and weapon, which isn't great when playing.
)

(event EventTick
  (params (DeltaSeconds :type Float%20%28single-precision%29))
  (bind _returnvalue (Utilities|Time|GetWorldDeltaSeconds))
  (bind _rotation_speed (Variables|InfimaGames|Casing|GetRotation%20Speed))
  (bind _returnvalue_2 (* _returnvalue _rotation_speed))
  (|CallParentFunction DeltaSeconds)
  (Utilities|FlowControl|Sequence
    (:then_0
      (if (Variables|InfimaGames|Casing|GetRotate)
        (Transformation|AddLocalRotation (Variables|Default|GetMesh) (Math|Rotator|MakeRotator _returnvalue_2 _returnvalue_2 0.0) false false)))
    (:then_1
      (if (>= (Actor|GetGameTimeSinceCreation) (Variables|InfimaGames|Data|GetDestroy%20Delay))
        (Actor|DestroyActor)))))

(fn ConstructionScript
  (|CallParentFunction))