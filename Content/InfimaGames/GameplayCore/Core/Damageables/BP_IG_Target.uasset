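; BP_IG_Target is a destructible target that reports itself as both an aim-assist target and a player enemy.
; Its construction script registers a child anchor field actor as an initialization field on the DestructibleTarget component.
; On any damage, it sends a hitmarker message to the damage causer, with no health or damage tracking in its own graph.
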(event Game|Damage|EventAnyDamage
  (params (Damage :type Float%20%28single-precision%29) (DamageType :type Damage%20Type%20Object%20Reference) (InstigatedBy :type Controller%20Object%20Reference) (DamageCauser :type Actor%20Object%20Reference))
  ;[0.5424 1 0.6286 1 12] Damage
  (Class|BPIIGCharacter|SpawnHitmarker(Message) DamageCauser))

(fn ConstructionScript
  (bind _asfield_system_actor (Utilities|Casting|CastToFieldSystemActor (Variables|/Script/Engine.ChildActorComponent|GetChildActor (Variables|Default|GetFS_AnchorField_Generic))))
  (Utilities|Array|AddUnique (Variables|/Script/GeometryCollectionEngine.GeometryCollectionComponent|GetInitializationFields (Variables|Default|GetDestructible%20Target)) _asfield_system_actor))

(fn IsAssistTarget
  (return true))

(fn IsPlayerEnemy
  (return true))