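; Default player camera manager that limits the view's yaw and pitch range for the controlled pawn.
; It applies its default clamps on BeginPlay, then each tick queries the pawn through GetClampsMessage for either the default or custom clamps.
; SetClampsFromValue writes the view yaw and pitch limits, keeping requested values within the default range so pawns cannot widen it.
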(event EventTick
  (params (DeltaSeconds :type Float%20%28single-precision%29))
  (|CallParentFunction DeltaSeconds)
  (Utilities|IsValid (Pawn|GetControlledPawn (Game|Player|GetOwningPlayerController))
    (:Is%20Valid
      (bind (_use_default _value) (Class|BPIIGCameraManagerTarget|GetClamps(Message) (Pawn|GetControlledPawn (Game|Player|GetOwningPlayerController))))
      (CallFunction|SetClampsfromValue (select _use_default (Variables|Default|GetClamps%20Default) _value)))))

(event EventBeginPlay
  (|CallParentFunction)
  (CallFunction|SetClampsfromValue (Variables|Default|GetClamps%20Default)))

(fn ConstructionScript)

(fn SetClampsfromValue
  (params (Value :type S%20Clamps%20Structure))
  (bind _clamps_default (Variables|Default|GetClamps%20Default))
  (bind _clamps_default_2 (Variables|Default|GetClamps%20Default))
  (bind _clamps_default_3 (Variables|Default|GetClamps%20Default))
  (bind _clamps_default_4 (Variables|Default|GetClamps%20Default))
  (bind _clampspitch (Utilities|Struct|BreakSClamps _clamps_default))
  (bind _clampsyaw (Utilities|Struct|BreakSClamps _clamps_default_2))
  (bind _clampsyaw_2 (Utilities|Struct|BreakSClamps _clamps_default_3))
  (bind _clampspitch_2 (Utilities|Struct|BreakSClamps _clamps_default_4))
  (bind (_x _y) (Math|Vector2D|BreakVector2D _clampspitch_2))
  (bind (_x_2 _y_2) (Math|Vector2D|BreakVector2D _clampspitch))
  (bind (_x_3 _y_3) (Math|Vector2D|BreakVector2D _clampsyaw))
  (bind (_x_4 _y_4) (Math|Vector2D|BreakVector2D _clampsyaw_2))
  (Utilities|FlowControl|Sequence
    (:then_0
      (Variables|Default|SetViewYawMin (Math|Float|ClampAngle (.X (Math|Vector2D|BreakVector2D (Utilities|Struct|BreakSClamps Value))) _x_4 _y_4))
      (Variables|Default|SetViewYawMax (Math|Float|ClampAngle (.Y (Math|Vector2D|BreakVector2D (Utilities|Struct|BreakSClamps Value))) _x_3 _y_3))
      (Variables|Default|SetViewPitchMin (Math|Float|ClampAngle (.X (Math|Vector2D|BreakVector2D (Utilities|Struct|BreakSClamps Value))) _x _y))
      (Variables|Default|SetViewPitchMax (Math|Float|ClampAngle (.Y (Math|Vector2D|BreakVector2D (Utilities|Struct|BreakSClamps Value))) _x_2 _y_2)))
    (:then_1
      (return))))