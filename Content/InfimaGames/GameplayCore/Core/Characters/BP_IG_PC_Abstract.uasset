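; Base player controller for Infima Games characters that handles spawning and respawning of the player's pawn.
; On BeginPlay, outside dedicated servers, it calls ServerSpawn, which destroys any controlled pawn, restarts the player through the game mode and adds a cover widget to the viewport.
; A separate server event forwards custom spawn requests with loadout, inventory data and attachment overrides to the game mode as a message.
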(event Custom|Event%20%28Server%29%20Spawn%20Player%20Custom
  (params (Override%20Attachments :type Boolean) (Loadout :type S%20IG%20Loadout%20Structure) (Inventory%20Data :type Data%20Table%20Object%20Reference))
  ;[1 0.9481 0 1 12] Spawn Player
  (Class|BPIIGGM|SpawnPlayerCustom(Message) (Game|GetGameMode) self Inventory%20Data Override%20Attachments Loadout))

(event Custom|Event%20Server%20Spawn
  ;[1 0.4061 0 1 12] Spawn
  (Utilities|FlowControl|Sequence
    (:then_0
      (Utilities|IsValid (Pawn|GetControlledPawn)
        (:Is%20Valid
          (Actor|DestroyActor (Pawn|GetControlledPawn)))))
    (:then_1
      (Class|GameModeBase|RestartPlayer (Game|GetGameMode) self)
      (bind _returnvalue (UserInterface|CreateWidget "/Game/InfimaGames/GameplayCore/Core/Widgets/WBP_IG_Cover.WBP_IG_Cover_C" self))
      (UserInterface|Viewport|AddtoViewport _returnvalue 0))))

(event EventBeginPlay
  ;[0.9123 1 0 1 12] Begin Play
  (if (not (Networking|IsDedicatedServer))
    (CallFunction|EventServerSpawn)))

(fn ConstructionScript)